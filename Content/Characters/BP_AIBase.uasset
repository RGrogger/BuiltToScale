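; BP_AIBase is an actor, named as an AI base, that the player consumes on contact to gain weight.
; When its Sphere overlaps a PlayerCharacter_Custom, a DoOnce gate adds WeightValue to the player's Weight and passes the new total to the HUD's calorie count.
; It then spawns the NS_Arrow_Hit Niagara effect at the player's location and destroys itself.
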(event `self.Sphere.OnComponentBeginOverlap`
  (params (OverlappedComponent :type "PrimitiveComponent Object Reference") (OtherActor :type "Actor Object Reference") (OtherComp :type "PrimitiveComponent Object Reference") (OtherBodyIndex :type Integer) (bFromSweep :type Boolean) (SweepResult :type "HitResult Structure (by ref)"))
  (bind _asplayer_character_custom (cast `/Game/Core/PlayerCharacter_Custom` OtherActor))
  (`/Engine/EditorBlueprintResources/StandardMacros.DoOnce` false
    (:`Completed`
      (bind _output_get (set `/Game/Core/PlayerCharacter_Custom.Weight` (+ (`/Game/Core/PlayerCharacter_Custom.Weight` _asplayer_character_custom) (`self.WeightValue`)) _asplayer_character_custom))
      (`/Game/UI/HUD_Custom.UpdateCalorieCount` (`/Game/Core/PlayerCharacter_Custom.HUDRef` _asplayer_character_custom) _output_get)
      (`NiagaraFunctionLibrary.SpawnSystemAtLocation` "/Game/Vefects/Anime_VFX/Shared/Skills/NS_Arrow_Hit.NS_Arrow_Hit" (`self.K2_GetActorLocation` _asplayer_character_custom))
      (`self.K2_DestroyActor`))))

(fn `UserConstructionScript`)