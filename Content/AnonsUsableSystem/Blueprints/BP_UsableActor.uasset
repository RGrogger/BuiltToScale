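; BP_UsableActor is a scene component that makes its owner a usable, inspectable or physics-driven object such as a key or lockable door.
; UseEvent plays a sound, then stores key IDs in the usable system, messages the owner or toggles locking, optionally destroying the owner.
; BeginPlay configures a physics constraint, spawning one if missing, and binds velocity-scaled impact sounds.
; A looping timer watches angle limits to play sounds and trigger linked usable actors.
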(event `UpdateInfo`
  (params (UsableSystem :type "/Game/AnonsUsableSystem/Blueprints/BP_UsableSystem Object Reference"))
  ;[0 0 0] Send info
  (`/Engine/EditorBlueprintResources/StandardMacros.IsValid` UsableSystem
    (:`Is Valid`
      (set `self.UsableReference` UsableSystem))
    (:`Is Not Valid`
      (`/Engine/EditorBlueprintResources/StandardMacros.IsValid` (`self.UsableReference`)
        (:`Is Valid`
          _))))
  (`/Game/AnonsUsableSystem/Blueprints/BP_UsableSystem.PhysicsItemInfoEvent` (`self.UsableReference`) (`self.UseText`) (`self.IsInspectable?`) self)
  (`/Game/AnonsUsableSystem/Blueprints/BP_UsableSystem.CreatePostProcess ` (`self.UsableReference`) (`self.OutlineColor`)))

(event `UseEvent`
  (params (`Use?` :type Boolean) (Actor :type "Actor Object Reference") (`IsUsable?` :type Boolean) (`IsKey?` :type Boolean))
  ;[0 0 0] CanAddCustomFunctionsHere
  (`GameplayStatics.PlaySoundAtLocation` (`self.OnUseSound`) (`Actor.K2_GetActorLocation` (`self.GetOwner`)) (struct) 5.0 1.0 0.0 null null null null) ; Use
  (if (`self.IsInspectable?`)
    (if `IsUsable?`
      (message `/Game/AnonsUsableSystem/Blueprints/BPI_UsableInterface.Usable` (`self.GetOwner`) true Actor false false :!label _label)
      (if (`self.IsDestroyedOnUse?`) :!label _label_2
        (if (`self.IsUsable?`)
          (`Actor.K2_DestroyActor` (`self.GetOwner`)))
        (else
          ;[0 1 0.1488] Lockable
          (`self.Lockable` `IsKey?` :!label _label_3)
          ;[0.09896 0.09896 0.09896] UpdateInfo
          (`self.UpdateInfo` (`self.UsableReference`))))
      (else
        (goto _label_3)))
    (elif (not (`self.IsKey?`))
      (if (`self.IsLocked?`)
        (`self.KeyCheck`
          (:`then`
            (goto _label_3))
          (:`Is Not Valid`
            (goto _label)))
        (else
          (goto _label)))
      (else
        ;;[0.9984 1 0.3542] AddKeyToArray
        (`KismetSystemLibrary.PrintString` "KeySaved" (`self.ShowDebug?`) false (struct :`G` 0.486931 :`B` 1.0 :`A` 1.0))
        (`KismetArrayLibrary.Array_Add` (`/Game/AnonsUsableSystem/Blueprints/BP_UsableSystem.Keys` (`self.UsableReference`)) (`self.LockOrKeyID`))
        (goto _label_2)))))

(event `OnActorHit_Event`
  (params (SelfActor :type "Actor Object Reference") (OtherActor :type "Actor Object Reference") (NormalImpulse :type "Vector Structure") (Hit :type "HitResult Structure (by ref)"))
  (bind _primitivereference (`self.PrimitiveReference`))
  (bind _returnvalue (/ (`KismetMathLibrary.VSize` (`self.GetComponentVelocity` _primitivereference)) 50.0))
  ;[0 1 0.1488] ImpactSound
  (if (> _returnvalue 0.1)
    (`KismetSystemLibrary.PrintString` (`KismetStringLibrary.Conv_DoubleToString` _returnvalue) (`self.ShowDebug?`) false (struct :`G` 0.039857 :`B` 1.0 :`A` 1.0) 5.0))
  (if (> _returnvalue (`self.ImpactTolerance`))
    (`/Engine/EditorBlueprintResources/StandardMacros.DoOnce` false :!label _label_4
      (:`Completed`
        (`GameplayStatics.PlaySoundAtLocation` (`self.ImpactSound`) Hit_Location (`KismetMathLibrary.Conv_VectorToRotator` Hit_Normal) (`KismetMathLibrary.MapRangeClamped` _returnvalue 1.0 20.0 1.0 5.0) (/ (`PrimitiveComponent.GetMass` _primitivereference) -100.0) 0.3 "/Game/AnonsUsableSystem/Demo/Audio/SoundAttenuation.SoundAttenuation" null null null)
        (`KismetSystemLibrary.Delay` 0.1)
        (goto _label_4 :!via `Reset`)))))

(event `self.ReceiveBeginPlay`
  (bind (_returnvalue_roll _returnvalue_pitch _returnvalue_yaw) (`KismetMathLibrary.BreakRotator` (`self.K2_GetComponentRotation`)))
  ;[0 1 0.03437] EventBeginPlay
  (set `self.UseText` (`self.InteractionText`))
  ;[0.9984 1 0.3542] PhysicsConstraintSettings
  (`self.ConstraintSettings`)
  ;[0 1 0.1488] ImpactSound
  (`/Engine/EditorBlueprintResources/StandardMacros.IsValid` (`self.ImpactSound`)
    (:`Is Valid`
      (`/Engine/EditorBlueprintResources/StandardMacros.IsValid` (`self.PrimitiveReference`)
        (:`Is Valid`
          (`PrimitiveComponent.SetNotifyRigidBodyCollision` (`self.PrimitiveReference`) true :!label _label_5)
          (add `Actor.OnActorHit` (`self.GetOwner`) (delegate `OnActorHit_Event`)))
        (:`Is Not Valid`
          (bind _asprimitive_component (cast `PrimitiveComponent` (`self.GetAttachParent`))
            (:`then`
              (set `self.PrimitiveReference` _asprimitive_component)
              (goto _label_5))
            (:`CastFailed`
              (`KismetSystemLibrary.PrintString` "PrimitiveComponent not valid" (`self.ShowDebug?`) false))))))
    (:`Is Not Valid`
      _))
  (`|ExecutionSequence`
    (:`then_0`
      (goto _label_3))
    (:`then_1`
      ;[0 0 0] AngleEventTimer
      (if (or (`KismetArrayLibrary.Array_IsValidIndex` (`self.AngleEventActors`)) (`KismetSystemLibrary.IsValid` (`self.AngleLimitSound`)))
        (bind _returnvalue (`KismetSystemLibrary.K2_SetTimerDelegate` (delegate `AngleEvent`) (`self.AngleLimitRate`) true))
        (set `self.InitAngle` (select `/Game/AnonsUsableSystem/Blueprints/Enum/E_axis` (`self.PhysicsAngleAxis`) :`NewEnumerator0` _returnvalue_roll :`NewEnumerator1` _returnvalue_pitch :`NewEnumerator2` _returnvalue_yaw :!type "Float (double-precision)"))
        (set `self.Timer` _returnvalue)))
    (:`then_2`
      (if (`self.IsPhysics?`)
        (`/Engine/EditorBlueprintResources/StandardMacros.IsValid` (`self.PrimitiveReference`)
          (:`Is Valid`
            _)
          (:`Is Not Valid`
            (bind _asprimitive_component_2 (cast `PrimitiveComponent` (`self.GetAttachParent`)))
            (set `self.PrimitiveReference` _asprimitive_component_2)))
        (`PrimitiveComponent.WakeAllRigidBodies` (`self.PrimitiveReference`))))))

(event `AngleEvent`
  (bind _returnvalue (`self.K2_GetComponentLocation`))
  (bind (_returnvalue_roll _returnvalue_pitch _returnvalue_yaw) (`KismetMathLibrary.BreakRotator` (`self.K2_GetComponentRotation`)))
  (bind _angleeventactors (`self.AngleEventActors`))
  (bind _anglelimitevent2 (`self.AngleLimitEvent2`))
  (bind _anglelimitevent (`self.AngleLimitEvent`))
  (bind _returnvalue_2 (`KismetArrayLibrary.Array_IsValidIndex` _angleeventactors))
  (bind _returnvalue_3 (- (select `/Game/AnonsUsableSystem/Blueprints/Enum/E_axis` (`self.PhysicsAngleAxis`) :`NewEnumerator0` _returnvalue_roll :`NewEnumerator1` _returnvalue_pitch :`NewEnumerator2` _returnvalue_yaw :!type "Float (double-precision)") (- (`self.InitAngle`) (`self.PhysicsAngleOffset`))))
  ;[0 0 0] AngleEventTimer
  (if (and (`KismetMathLibrary.NearlyEqual_FloatFloat` _anglelimitevent _returnvalue_3 10.0) (!= _anglelimitevent 0.0))
    (`|ExecutionSequence`
      (:`then_0`
        (`/Engine/EditorBlueprintResources/StandardMacros.DoOnce` true :!label _label_6
          (:`Completed`
            ;;[0.779 1 0.3783] AngleSoundTimer
            (`/Engine/EditorBlueprintResources/StandardMacros.IsValid` (`self.AngleLimitSound`)
              (:`Is Valid`
                (`GameplayStatics.PlaySoundAtLocation` (`self.AngleLimitSound`) _returnvalue (struct) 5.0 1.0 0.0 null null null null))
              (:`Is Not Valid`
                _))
            (if _returnvalue_2
              (for _array_element _angleeventactors
                (`/Engine/EditorBlueprintResources/StandardMacros.IsValid` _array_element
                  (:`Is Valid`
                    (bind _returnvalue_4 (`Actor.GetComponentByClass` _array_element "BP_UsableActor_C"))
                    (if (`KismetSystemLibrary.IsValid` _returnvalue_4)
                      (`self.UseEvent` _returnvalue_4 true null false true)))))))))
      (:`then_1`
        (goto _label_7 :!via `Reset`)))
    (elif (and (or (`KismetMathLibrary.NearlyEqual_FloatFloat` _anglelimitevent2 _returnvalue_3 10.0) (>= _returnvalue_3 300.0)) (!= _anglelimitevent2 0.0))
      (`|ExecutionSequence`
        (:`then_0`
          (goto _label_6 :!via `Reset`))
        (:`then_1`
          (`/Engine/EditorBlueprintResources/StandardMacros.DoOnce` true :!label _label_7
            (:`Completed`
              (`/Engine/EditorBlueprintResources/StandardMacros.IsValid` (`self.AngleLimitSound`)
                (:`Is Valid`
                  (`GameplayStatics.PlaySoundAtLocation` (`self.AngleLimitSound2`) _returnvalue (struct) 5.0 1.0 0.0 null null null null))
                (:`Is Not Valid`
                  _))
              (if _returnvalue_2
                (for _array_element_2 _angleeventactors
                  (`/Engine/EditorBlueprintResources/StandardMacros.IsValid` _array_element_2
                    (:`Is Valid`
                      (bind _returnvalue_5 (`Actor.GetComponentByClass` _array_element_2 "BP_UsableActor_C"))
                      (if (`KismetSystemLibrary.IsValid` _returnvalue_5)
                        (`self.UseEvent` _returnvalue_5 true null false true))))))))))
      (else
        (goto _label_6 :!via `Reset`)))))

(fn `ConstraintSettings`
  (bind _physicsdistencelimit (`self.PhysicsDistenceLimit`))
  (bind _physicsanglelimit (`self.PhysicsAngleLimit`))
  (bind _constraintreference (`self.ConstraintReference`))
  (bind _physicsangleoffset (`self.PhysicsAngleOffset`))
  (bind _physicsangleaxis (`self.PhysicsAngleAxis`))
  ;[0.9984 1 0.3542] PhysicsConstraintSettings
  (if (`self.EnableConstraints`)
    (`/Engine/EditorBlueprintResources/StandardMacros.IsValid` (`self.ConstraintReference`)
      (:`Is Valid`
        (`PhysicsConstraintComponent.SetConstrainedComponents` (`self.ConstraintReference`) (`self.PrimitiveReference`) "None" null "None" :!label _label)
        (`PrimitiveComponent.WakeAllRigidBodies` (`self.PrimitiveReference`))
        (switch `/Game/AnonsUsableSystem/Blueprints/Enum/E_axis` (`self.PhysicsAngleAxis`)
          (:`NewEnumerator3`
            _)
          (:`NewEnumerator0`
            ;;[1 1 1] Rotation
            (`PhysicsConstraintComponent.SetAngularTwistLimit` _constraintreference "ACM_Limited" _physicsanglelimit))
          (:`NewEnumerator1`
            (`PhysicsConstraintComponent.SetAngularSwing2Limit` _constraintreference "ACM_Limited" _physicsanglelimit))
          (:`NewEnumerator2`
            (`PhysicsConstraintComponent.SetAngularSwing1Limit` _constraintreference "ACM_Limited" _physicsanglelimit)))
        (switch `/Game/AnonsUsableSystem/Blueprints/Enum/E_axis` (`self.PhysicsDistenceAxis`)
          (:`NewEnumerator3`
            _)
          (:`NewEnumerator0`
            ;;[1 1 1] Location
            (`PhysicsConstraintComponent.SetLinearXLimit` _constraintreference "LCM_Limited" _physicsdistencelimit))
          (:`NewEnumerator1`
            (`PhysicsConstraintComponent.SetLinearYLimit` _constraintreference "LCM_Limited" _physicsdistencelimit))
          (:`NewEnumerator2`
            (`PhysicsConstraintComponent.SetLinearZLimit` _constraintreference "LCM_Limited" _physicsdistencelimit)))
        (if (!= _physicsangleoffset 0.0)
          (`PhysicsConstraintComponent.SetConstraintReferenceFrame` (`self.ConstraintReference`) "Frame1" (`KismetMathLibrary.MakeTransform` (0.0 0.0 0.0) (`KismetMathLibrary.MakeRotator` (`KismetMathLibrary.SelectFloat` _physicsangleoffset 0.0 (`|EnumEquality` _physicsangleaxis "NewEnumerator0")) (`KismetMathLibrary.SelectFloat` _physicsangleoffset 0.0 (`|EnumEquality` _physicsangleaxis "NewEnumerator1")) (`KismetMathLibrary.SelectFloat` _physicsangleoffset 0.0 (`|EnumEquality` _physicsangleaxis "NewEnumerator2"))))))
        (return))
      (:`Is Not Valid`
        (`/Engine/EditorBlueprintResources/StandardMacros.IsValid` (`self.PrimitiveReference`)
          (:`Is Valid`
            (bind _returnvalue (`|SpawnActorFromClass` (`self.PhysicsConstraint`) (`self.K2_GetComponentToWorld`) "AlwaysSpawn" "OverrideRootScale" (`self.GetOwner`) null :!label _label_2))
            (set `self.ConstraintReference` (`Actor.GetComponentByClass` _returnvalue "/Script/Engine.PhysicsConstraintComponent"))
            (goto _label))
          (:`Is Not Valid`
            (bind _asprimitive_component (cast `PrimitiveComponent` (`self.GetAttachParent`))
              (:`then`
                (set `self.PrimitiveReference` _asprimitive_component)
                (goto _label_2))
              (:`CastFailed`
                _)))))))
  (return))

(fn `Lockable`
  (params (Condition :type Boolean))
  (bind _returnvalue (`self.K2_GetComponentLocation`))
  (bind _showdebug_ (`self.ShowDebug?`))
  (bind _primitivereference (`self.PrimitiveReference`))
  (bind _primitivereference_2 (`self.PrimitiveReference`))
  (bind _returnvalue_2 (`KismetSystemLibrary.MakeLiteralText` (`self.InteractionText`)))
  (bind _rootcomponent (`Actor.RootComponent` (`self.GetOwner`)))
  (bind _returnvalue_3 (and (== (`self.K2_GetComponentRotation` _primitivereference_2) (`self.K2_GetComponentRotation` _rootcomponent) :`ErrorTolerance` 2.0) (== (`self.K2_GetComponentLocation` _primitivereference_2) (`self.K2_GetComponentLocation` _rootcomponent) :`ErrorTolerance` 2.0)))
  (if (`self.IsLockable?`)
    (if Condition
      (if _returnvalue_3
        (if (`self.IsLocked?`) :!label _label
          (set `self.IsLocked?` false)
          (set `self.IsPhysics?` true)
          (`PrimitiveComponent.SetSimulatePhysics` _primitivereference true)
          (`KismetSystemLibrary.PrintString` "Unlocked" _showdebug_ false)
          (`GameplayStatics.PlaySoundAtLocation` (`self.UnlockedSound`) _returnvalue (struct) 1.0 1.0 0.0 null null null null) ; UnLocked
          (else
            (set `self.IsLocked?` true)
            (set `self.IsPhysics?` false)
            (`PrimitiveComponent.SetSimulatePhysics` _primitivereference false)
            (`KismetSystemLibrary.PrintString` "Locked" _showdebug_ false)
            (`GameplayStatics.PlaySoundAtLocation` (`self.LockedSound`) _returnvalue (struct) 1.0 1.0 0.0 null null null null) ; Locked
          ))
        (set `self.UseText` (select `bool` (`self.IsLocked?`) :`false` (`|FormatText` "{a} {b}" _returnvalue_2 "(Unlocked)") :`true` (`|FormatText` "{a} {b}" _returnvalue_2 "(Locked)")) :!label _label_2)
        (else
          (`KismetSystemLibrary.PrintString` "Error: is open" _showdebug_ false :!label _label_3)
          (if (`self.IsLockable?`) :!label _label_4
            (`/Engine/EditorBlueprintResources/StandardMacros.IsValid` (`self.PrimitiveReference`)
              (:`Is Valid`
                _)
              (:`Is Not Valid`
                (bind _asprimitive_component (cast `PrimitiveComponent` (`self.GetAttachParent`)))
                (set `self.PrimitiveReference` _asprimitive_component)))
            (`PrimitiveComponent.SetSimulatePhysics` (`self.PrimitiveReference`) (not (`self.IsLocked?`)))
            (goto _label_2)
            (else
              _))))
      (elif _returnvalue_3
        (`self.KeyCheck`
          (:`then`
            (goto _label))
          (:`Is Not Valid`
            (`KismetSystemLibrary.PrintString` "Error: no matching key found" _showdebug_ false)
            (goto _label_4)))
        (else
          (goto _label_3)))))
  (return))