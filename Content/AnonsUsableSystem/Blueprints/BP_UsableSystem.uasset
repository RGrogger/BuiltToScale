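; Player scene component for highlighting and using objects, and for grabbing, rotating, throwing and pushing or pulling physics props.
; Each tick it traces from the camera for BP_UsableActor components, setting custom-depth highlights and managing a use-prompt widget.
; Key-filtered use starts a hold timer that grabs simulating objects through the owner's PhysicsHandle.
; While grabbing, the component moves itself along the screen-center ray as the handle's target, with optional mass-based angular damping.
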(event `self.ReceiveTick`
  (params (DeltaSeconds :type "Float (single-precision)"))
  (set `self.TargetLocation` (`self.K2_GetComponentLocation`))
  (`self.LineTrace`))

(event `ResetTimer`
  (bind _returnvalue (`Actor.GetComponentByClass` (`self.GetOwner`) "/Script/Engine.PhysicsHandleComponent"))
  ;[0 0 0] BeginPlay
  (`KismetSystemLibrary.PrintString` (`KismetStringLibrary.Conv_DoubleToString` (`self.LineTraceRate`)) (`self.ShowDebug?`) false)
  ;[0 0 0] SetsDistance
  (`/Engine/EditorBlueprintResources/StandardMacros.DoOnce` false :!label _label
    (:`Completed`
      (set `self.CurrentDistance` (`self.BaseDistance`))
      ;[0 0 0] Checks to see if player has a physics handle
      (`KismetSystemLibrary.Delay` 0.2)
      (`/Engine/EditorBlueprintResources/StandardMacros.IsValid` (`self.PhysicsHandle`)
        (:`Is Not Valid`
          (if (`KismetSystemLibrary.IsValid` _returnvalue)
            (set `self.PhysicsHandle` _returnvalue)
            (`PhysicsHandleComponent.SetInterpolationSpeed` (`self.PhysicsHandle`) 20.0)
            (else
              (`KismetSystemLibrary.PrintString` "PhysicsHandle not found in player chararcter BP" (`self.ShowDebug?`) false (struct :`R` 1.0 :`G` 0.014146 :`A` 1.0)))))))))

(event `PhysicsItemInfoEvent`
  (params (InteractionText :type "Text (by ref)") (`IsInspection?` :type Boolean) (UsableActorComponent :type "/Game/AnonsUsableSystem/Blueprints/BP_UsableActor Object Reference"))
  (bind _usewidget (`self.UseWidget`))
  (bind _usewidget_2 (`self.UseWidget`))
  (bind _ac_usableactor (`self.AC_UsableActor`))
  ;[0 0 0] Create Use Widget
  (`|ExecutionSequence`
    (:`then_0`
      (`/Engine/EditorBlueprintResources/StandardMacros.IsValid` _usewidget_2 :!label _label_2
        (:`Is Valid`
          (`Widget.RemoveFromParent` _usewidget_2)
          (goto _label_3 :!via `Reset`))
        (:`Is Not Valid`
          (goto _label_3 :!via `Reset`))))
    (:`then_1`
      (if (== UsableActorComponent _ac_usableactor)
        (`/Engine/EditorBlueprintResources/StandardMacros.IsValid` (`self.HighlightedObject`)
          (:`Is Valid`
            (set `self.UseText` InteractionText))
          (:`Is Not Valid`
            (goto _label_2)))
        (else
          (set `self.UseText` (`/Game/AnonsUsableSystem/Blueprints/BP_UsableActor.UseText` _ac_usableactor))))
      (`/Engine/EditorBlueprintResources/StandardMacros.DoOnce` true :!label _label_3
        (:`Completed`
          (`/Engine/EditorBlueprintResources/StandardMacros.IsValid` _usewidget
            (:`Is Valid`
              (`Widget.RemoveFromParent` _usewidget))
            (:`Is Not Valid`
              _))
          (`self.CreateUseWidget` (`self.UseText`)))))))

(event `self.ReceiveBeginPlay`
  ;[0 0 0] BeginPlay
  (goto _label))

(event `LineTrace`
  (bind _physicshandle (`self.PhysicsHandle`))
  ;[0 0 0] BeginPlay
  (if (`self.ShouldTrace?`)
    ;;[0 0 0] Create Linetrace and update physics location
    (`self.CreateLinetrace`)
    ;;[0 0 0] SetsPhysicsLocation
    (if (`self.IsGrabbed?`)
      (`/Engine/EditorBlueprintResources/StandardMacros.IsValid` _physicshandle
        (:`Is Valid`
          (`PhysicsHandleComponent.SetTargetLocation` _physicshandle (`self.K2_GetComponentLocation`)))
        (:`Is Not Valid`
          _)))
    ;[0 0 0] Create Use Widget
    (if (`self.IsGrabbed?`)
      (goto _label_2)
      (else
        (`/Engine/EditorBlueprintResources/StandardMacros.IsValid` (`self.HighlightedObject`)
          (:`Is Not Valid`
            (goto _label_2)))))))

(event `Use`
  (params (Use :type Boolean) (PhysicsHandle :type "PhysicsHandleComponent Object Reference"))
  (bind _showdebug_ (`self.ShowDebug?`))
  (bind _ac_usableactor (`self.AC_UsableActor`))
  (bind _grabobject (`self.GrabObject`))
  (bind _grabobject_2 (`self.GrabObject`))
  (bind _physicshandle (`self.PhysicsHandle`))
  (bind _ac_usableactor_2 (`self.AC_UsableActor`))
  (bind _ac_usableactor_3 (`self.AC_UsableActor`))
  (bind _ac_usableactor_4 (`self.AC_UsableActor`))
  (bind _grabsound (`/Game/AnonsUsableSystem/Blueprints/BP_UsableActor.GrabSound` _ac_usableactor))
  (bind _releasesound (`/Game/AnonsUsableSystem/Blueprints/BP_UsableActor.ReleaseSound` _ac_usableactor_3))
  ;[0 0 0] Use
  (if Use
    (`/Engine/EditorBlueprintResources/StandardMacros.IsValid` (`self.PhysicsHandle`)
      (:`Is Valid`
        _)
      (:`Is Not Valid`
        (set `self.PhysicsHandle` PhysicsHandle)))
    ;;[0.2217 1 0] PhysicsGrab
    (if (`KismetSystemLibrary.IsValid` _ac_usableactor_4)
      (`KismetSystemLibrary.PrintString` (`KismetStringLibrary.Concat_StrStr` "Usable is: " (`KismetStringLibrary.Conv_BoolToString` (`/Game/AnonsUsableSystem/Blueprints/BP_UsableActor.IsUsable?` _ac_usableactor_4))) (`self.ShowDebug?`) false))
    (`/Engine/EditorBlueprintResources/StandardMacros.IsValid` _grabobject
      (:`Is Valid`
        (`PrimitiveComponent.WakeAllRigidBodies` (`self.GrabObject`))
        (bind _returnvalue (`KismetSystemLibrary.K2_SetTimerDelegate` (delegate `PhysicsPickupEvent`) (`self.GrabDelay`)))
        (set `self.PhysicsTimer` _returnvalue)
        (set `self.IsHoldingKey?` false)
        (if (`self.IsSimulatingPhysics` _grabobject (`self.HitBone`))
          (`KismetSystemLibrary.PrintString` (`KismetStringLibrary.Concat_StrStr` "Is Holding: " (`KismetStringLibrary.Conv_BoolToString` (`self.IsHoldingKey?`))) (`self.ShowDebug?`) false)
          (goto _label_5 :!via `Reset`))))
    (else
      ;;[0.2217 1 0] PhysicsReleases
      (`KismetSystemLibrary.K2_ClearAndInvalidateTimerHandle` (`self.PhysicsTimer`) :!label _label_4)
      (if (`self.IsGrabbed?`)
        (set `self.LineTraceRate` (`self.LineTraceRate`))
        (`/Engine/EditorBlueprintResources/StandardMacros.IsValid` _physicshandle
          (:`Is Valid`
            (`/Engine/EditorBlueprintResources/StandardMacros.IsValid` (`self.GrabObject`)
              (:`Is Valid`
                (`self.ResetTimer`)
                (`PhysicsHandleComponent.SetInterpolationSpeed` _physicshandle 1.0)
                (if (`/Game/AnonsUsableSystem/Blueprints/BP_UsableActor.MassEffectsGrab?` (`self.AC_UsableActor`))
                  (`PrimitiveComponent.SetAngularDamping` (`PhysicsHandleComponent.GetGrabbedComponent` _physicshandle) (`self.GrabADamping`)))
                (set `self.IsGrabbed?` false)
                (set `self.IsHoldingKey?` false)
                (`PrimitiveComponent.SetPhysicsMaxAngularVelocityInDegrees` (`self.GrabObject`) 3400.0 false "None")
                (set `self.GrabObject` null)
                (`PhysicsHandleComponent.ReleaseComponent` _physicshandle)
                (`KismetSystemLibrary.PrintString` "Released" (`self.ShowDebug?`) false (struct :`R` 1.0 :`G` 0.014146 :`A` 1.0) 5.0)
                (set `self.CurrentDistance` (`self.BaseDistance`))
                (`/Engine/EditorBlueprintResources/StandardMacros.IsValid` _releasesound
                  (:`Is Valid`
                    (`GameplayStatics.PlaySoundAtLocation` _releasesound (`Actor.K2_GetActorLocation` (`self.GetOwner` _ac_usableactor_3)) (struct) 1.0 1.0 0.0 null null null null)))))))
        (else
          (`/Engine/EditorBlueprintResources/StandardMacros.IsValid` _ac_usableactor_2
            (:`Is Valid`
              (`/Game/AnonsUsableSystem/Blueprints/BP_UsableActor.UpdateInfo` _ac_usableactor_2 self))))))))

(event `PhysicsPickupEvent`
  (bind _showdebug_ (`self.ShowDebug?`))
  (bind _ac_usableactor (`self.AC_UsableActor`))
  (bind _grabobject (`self.GrabObject`))
  (bind _grabsound (`/Game/AnonsUsableSystem/Blueprints/BP_UsableActor.GrabSound` _ac_usableactor))
  ;[0 0 0] Use
  ;;[0.2217 1 0] PhysicsGrab
  (if (and (`self.IsSimulatingPhysics` (`self.GrabObject`) (`self.HitBone`)) (`/Game/AnonsUsableSystem/Blueprints/BP_UsableActor.IsPhysics?` (`self.AC_UsableActor`)))
    (`/Engine/EditorBlueprintResources/StandardMacros.IsValid` (`self.HighlightedObject`)
      (:`Is Valid`
        (set `self.IsHoldingKey?` true)
        (`KismetSystemLibrary.PrintString` (`KismetStringLibrary.Concat_StrStr` "Is Holding: " (`KismetStringLibrary.Conv_BoolToString` (`self.IsHoldingKey?`))) (`self.ShowDebug?`) false)
        (`/Engine/EditorBlueprintResources/StandardMacros.DoOnce` true :!label _label_5
          (:`Completed`
            (if (`KismetSystemLibrary.IsValid` (`self.PhysicsHandle`))
              (`KismetSystemLibrary.PrintString` "Grabbed" _showdebug_ false (struct :`R` 1.0 :`G` 0.014146 :`A` 1.0) 5.0)
              (set `self.LineTraceRate` (`self.LineTraceRate`))
              (`PrimitiveComponent.SetPhysicsMaxAngularVelocityInDegrees` (`self.GrabObject`) 0.0 false "None")
              (if (`/Game/AnonsUsableSystem/Blueprints/BP_UsableActor.MassEffectsGrab?` (`self.AC_UsableActor`))
                (set `self.GrabADamping` (`PrimitiveComponent.GetAngularDamping` _grabobject))
                (`PrimitiveComponent.SetAngularDamping` _grabobject (/ (`PrimitiveComponent.GetMass` (`self.GrabObject`)) 50.0)))
              (`PhysicsHandleComponent.GrabComponentAtLocation` (`self.PhysicsHandle`) (`self.GrabObject`) (`self.HitBone`) (`KismetSystemLibrary.GetComponentBounds` (`self.GrabObject`)))
              (`self.ResetTimer`)
              (`PhysicsHandleComponent.SetInterpolationSpeed` (`self.PhysicsHandle`) 5.0)
              (set `self.IsGrabbed?` true)
              (set `self.Temp` (- (`KismetSystemLibrary.GetComponentBounds` (`self.GrabObject`)) (`self.HitLocation`)))
              (set `self.CurrentDistance` (`KismetMathLibrary.Vector_Distance` (`KismetSystemLibrary.GetComponentBounds` (`self.GrabObject`)) (`self.K2_GetComponentLocation` (`/Game/Core/BP_PlayerCharacter_Crane.Camera` (cast `/Game/Core/BP_PlayerCharacter_Crane` (`self.GetOwner`) :!pure true)))))
              (`/Engine/EditorBlueprintResources/StandardMacros.IsValid` _grabsound
                (:`Is Valid`
                  (`GameplayStatics.PlaySoundAtLocation` _grabsound (`Actor.K2_GetActorLocation` (`self.GetOwner` _ac_usableactor)) (struct) 1.0 1.0 0.0 "/Game/AnonsUsableSystem/Demo/Audio/SoundAttenuation.SoundAttenuation" null null null)))
              (else
                (`KismetSystemLibrary.PrintString` "PhysicsHandle not found" _showdebug_ false)))))))
    (else
      (set `self.IsHoldingKey?` true))))

(event `Releases`
  ;[0 0 0] Use
  ;;[0.2217 1 0] PhysicsReleases
  (goto _label_4))

(fn `CreateLinetrace`
  (locals (NewLocalVar :type "Vector Structure"))
  (bind _returnvalue (`GameplayStatics.GetPlayerCameraManager` 0))
  (bind _highlightedobject (`self.HighlightedObject`))
  (bind (_sizex _sizey) (`PlayerController.GetViewportSize` (`GameplayStatics.GetPlayerController` 0)))
  (bind _returnvalue_2 (`PlayerCameraManager.GetCameraLocation` _returnvalue))
  ;[0 0 0] Create linetrace and highlight
  (if (not (`self.HasInspectStarted?`))
    (if (`self.IsGrabbed?`)
      (`self.K2_SetWorldLocation` (+ (* (`.WorldDirection` (`PlayerController.DeprojectScreenPositionToWorld` (`GameplayStatics.GetPlayerController` 0) (`KismetMathLibrary.Conv_IntToDouble` (/ _sizex 2)) (`KismetMathLibrary.Conv_IntToDouble` (/ _sizey 2)))) (`self.CurrentDistance`)) (+ (`Actor.K2_GetActorLocation` (`self.GetOwner`)) (`self.LineTraceLocationOffset`)) (`self.LineTraceDirectionOffset`) (`self.Temp`)))
      (else
        (bind (_outhit _returnvalue_3) (`KismetSystemLibrary.LineTraceSingle` _returnvalue_2 (+ _returnvalue_2 (* (`self.GetForwardVector` (`Actor.RootComponent` _returnvalue)) (`self.BaseDistance`))) "TraceTypeQuery1" true (`|MakeArray` (`self.GetOwner`)) (select `bool` (`self.ShowDebug?`) :`true` "ForDuration" :!type "EDrawDebugTrace Enum") false (struct :`R` 1.0 :`A` 1.0) (struct :`G` 1.0 :`A` 1.0) 1.0))
        (if _returnvalue_3
          (bind (_bblockinghit _binitialoverlap _time _distance _location _impactpoint _normal _impactnormal _physmat _hitactor _hitcomponent _hitbonename) (`GameplayStatics.BreakHitResult` _outhit))
          (bind _returnvalue_4 (`Actor.K2_GetComponentsByClass` _hitactor "/Game/AnonsUsableSystem/Blueprints/BP_UsableActor.BP_UsableActor_C"))
          (if (`KismetArrayLibrary.Array_IsValidIndex` _returnvalue_4)
            (for _array_element _returnvalue_4
              (if (== (`self.GetAttachParent` _array_element) _hitcomponent)
                (set `self.AC_UsableActor` _array_element)
                (set `self.HitLocation` _location)
                (set `self.HitBone` _hitbonename)
                (`/Engine/EditorBlueprintResources/StandardMacros.IsValid` _highlightedobject
                  (:`Is Valid`
                    (if (not (== (`self.GrabObject`) _hitcomponent))
                      (`PrimitiveComponent.SetRenderCustomDepth` _highlightedobject false)
                      (`PrimitiveComponent.SetRenderCustomDepth` _highlightedobject false)
                      (bind _output_get (set `self.HighlightedObject` _hitcomponent :!label _label))
                      (bind _output_get_2 (set `self.GrabObject` _output_get))
                      (`PrimitiveComponent.SetRenderCustomDepth` _output_get_2 true)
                      (`/Game/AnonsUsableSystem/Blueprints/BP_UsableActor.UpdateInfo` _array_element self)
                      (set `self.AC_UsableActor` _array_element)))
                  (:`Is Not Valid`
                    (goto _label)))
                (return)))))
        (`self.RemoveHighlight` :!label _label_2)
        (return)))
    (else
      (goto _label_2))))

(fn `CreateUseWidget`
  (params (UseTextLabel :type Text))
  ;[0 0 0] CreateUseWidget
  (`/Engine/EditorBlueprintResources/StandardMacros.IsValid` (`self.HighlightedObject`)
    (:`Is Valid`
      (bind _returnvalue (`|CreateWidget` "/Game/AnonsUsableSystem/UI/W_UseWidget.W_UseWidget_C" null UseTextLabel))
      (bind _output_get (set `self.UseWidget` _returnvalue))
      (`UserWidget.AddToPlayerScreen` _output_get 0))
    (:`Is Not Valid`
      _))
  (return))

(fn `PhysicsObjectDistance`
  (params (Distance :type "Float (double-precision)") (Min :type "Float (double-precision)" :default 300.0) (Max :type "Float (double-precision)" :default 600.0))
  ;[0 0 0] SetPhysicsDistance
  (if (== Distance 0.0)
    _
    (elif (`self.IsGrabbed?`)
      (set `self.CurrentDistance` (`KismetMathLibrary.FClamp` (+ (* Distance 5.0) (`self.CurrentDistance`)) Min Max)))))

(fn `PhysicsObjectRotate`
  (params (Lookup :type "Float (double-precision)") (Turn :type "Float (double-precision)"))
  (bind _ac_usableactor (`self.AC_UsableActor`))
  ;[0 0 0] RotatePhysicsObject
  (`/Engine/EditorBlueprintResources/StandardMacros.IsValid` _ac_usableactor
    (:`Is Valid`
      (if (`/Game/AnonsUsableSystem/Blueprints/BP_UsableActor.IsRotatable?` _ac_usableactor)
        (if (`self.IsGrabbed?`)
          (`self.K2_SetWorldRotation` (`self.GrabObject`) (`KismetMathLibrary.MakeRotator` (+ (* Lookup -1.0) (.roll (`self.K2_GetComponentRotation` (`self.GrabObject`)))) 0.0 (+ (* Turn -1.0) (.yaw (`self.K2_GetComponentRotation` (`self.GrabObject`))))) false true)
          ;[0.1198 0.1198 0.1198] Removes Angular Velocity
          (`/Engine/EditorBlueprintResources/StandardMacros.DoOnce` false
            (:`Completed`
              (`PrimitiveComponent.SetPhysicsAngularVelocityInDegrees` (`self.GrabObject`) (0.0 0.0 0.0) false (`self.HitBone`)))))))))

(fn `PhysicsObjectThrow`
  (params (ThrowStrength :type "Float (double-precision)" :default 1000.0))
  (bind _grabobject (`self.GrabObject`))
  (bind _ac_usableactor (`self.AC_UsableActor`))
  (bind (_returnvalue_roll _returnvalue_pitch _returnvalue_yaw) (`KismetMathLibrary.BreakRotator` (`Pawn.GetControlRotation` (`Actor.Instigator` (`self.GetOwner`)))))
  ;[0 0 0] ThrowPhysicsObject
  (if (`self.IsGrabbed?`)
    (if (`self.IsSimulatingPhysics` (`self.GrabObject`) "None")
      (set `self.IsHoldingKey?` false)
      (`/Engine/EditorBlueprintResources/StandardMacros.IsValid` _grabobject
        (:`Is Valid`
          (`PhysicsHandleComponent.ReleaseComponent` (`self.PhysicsHandle`))
          (`PrimitiveComponent.AddImpulse` _grabobject (* (`KismetMathLibrary.GetForwardVector` (`KismetMathLibrary.MakeRotator` 0.0 (+ _returnvalue_pitch 10.0) _returnvalue_yaw)) ThrowStrength) (`self.HitBone`) true)
          (set `self.IsGrabbed?` false)
          (set `self.GrabObject` null)
          (set `self.LineTraceRate` (`self.LineTraceRate`))
          (set `self.CurrentDistance` (`self.BaseDistance`))
          (`GameplayStatics.PlaySoundAtLocation` (`/Game/AnonsUsableSystem/Blueprints/BP_UsableActor.ThrowSound` _ac_usableactor) (`Actor.K2_GetActorLocation` (`self.GetOwner` _ac_usableactor)) (struct) 1.0 1.0 0.0 null null null null))))))

(fn `RemoveHighlight`
  (bind _highlightedobject (`self.HighlightedObject`))
  (`/Engine/EditorBlueprintResources/StandardMacros.IsValid` _highlightedobject
    (:`Is Valid`
      (`PrimitiveComponent.SetRenderCustomDepth` _highlightedobject false)
      (set `self.HighlightedObject` null)
      (`Widget.RemoveFromParent` (`self.UseWidget`)))))

(fn `SetWidgetVisibility`
  (params (Selection :type "ESlateVisibility Enum" :default "Visible"))
  (bind _usewidget (`self.UseWidget`))
  (`/Engine/EditorBlueprintResources/StandardMacros.IsValid` _usewidget
    (:`Is Valid`
      (`Widget.SetVisibility` _usewidget Selection))
    (:`Is Not Valid`
      _))
  (return))

(fn `UseFunction`
  (params (Use :type Boolean) (PhysicsHandle :type "PhysicsHandleComponent Object Reference") (Key :type "Key Structure" :default "None"))
  (bind _ac_usableactor (`self.AC_UsableActor`))
  (bind _usewidget (`self.UseWidget`))
  (`/Engine/EditorBlueprintResources/StandardMacros.IsValid` PhysicsHandle
    (:`Is Valid`
      (set `self.PhysicsHandle` PhysicsHandle))
    (:`Is Not Valid`
      _))
  (`/Engine/EditorBlueprintResources/StandardMacros.IsValid` _ac_usableactor
    (:`Is Valid`
      (if (`KismetArrayLibrary.Array_Contains` (`/Game/AnonsUsableSystem/Blueprints/BP_UsableActor.InteractionKeys` _ac_usableactor) Key)
        (`self.Use` Use (`self.PhysicsHandle`))
        (if Use
          (`/Engine/EditorBlueprintResources/StandardMacros.IsValid` _usewidget
            (:`Is Valid`
              (`Widget.RemoveFromParent` _usewidget))))))))