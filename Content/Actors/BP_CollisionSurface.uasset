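; BP_CollisionSurface is a trigger actor that sends the construction player character back to a checkpoint on contact.
; BeginPlay binds the box collision's overlap event, and BoxBeginOverlap filters for BP_PlayerCharacter_Construction before calling MovePlayerToCheckpoint on GameMode_Custom.
; Disconnected leftover nodes hold a generic Character check and a teleport that zeroes velocity and picks a random point around SurfaceActor's bounds.
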(fn `BoxBeginOverlap`
  (params (OverlappedComponent :type "PrimitiveComponent Object Reference") (OtherActor :type "Actor Object Reference") (OtherComp :type "PrimitiveComponent Object Reference") (OtherBodyIndex :type Integer) (bFromSweep :type Boolean) (SweepResult :type "HitResult Structure (by ref)"))
  (cast `/Game/Core/BP_PlayerCharacter_Construction` OtherActor)
  (bind _asgame_mode_custom (cast `/Game/Core/GameMode_Custom` (`GameplayStatics.GetGameMode`)))
  (`/Game/Core/GameMode_Custom.MovePlayerToCheckpoint` _asgame_mode_custom))

(fn `ReceiveBeginPlay`
  (add `PrimitiveComponent.OnComponentBeginOverlap` (`self.BoxCollision`) (`|CreateDelegate` :!event `BoxBeginOverlap`)))

(fn `UserConstructionScript`)