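; Actor component that runs a button-mashing challenge and reports success or failure through its Completed dispatcher.
; On BeginPlay it picks a random key and press target, then shows a WBP_SpamBar prompt with a progress bar.
; Matching presses fill the bar to win, while a retriggerable delay on release fails the player for pausing, as does never starting in time.
; Either outcome removes the widget and destroys the component.
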(event `self.ReceiveBeginPlay`
  (set `self.NeededAmount` (`KismetMathLibrary.RandomFloatInRange` 20.0 30.0))
  (bind _returnvalue (`|CreateWidget` "/Game/UI/WBP_SpamBar.WBP_SpamBar_C"))
  (bind _output_get (set `self.WidgetReference` _returnvalue))
  (`UserWidget.AddToViewport` _output_get 0)
  (bind _output_get_2 (set `self.KeyPressed` (select `int` (`KismetMathLibrary.RandomInteger` 3) :`0` "E" :`1` "Q" :`2` "F" :`3` "R" :!type "Key Structure")))
  (`TextBlock.SetText` (`/Game/UI/WBP_SpamBar.SpamText` (`self.WidgetReference`)) (`|FormatText` "Spam {Key}" (`KismetInputLibrary.Key_GetDisplayName` _output_get_2)))
  (`self.UpdateProgressBar`)
  (`KismetSystemLibrary.PrintString` "Hello")
  ;[0 0 0] If you dont start spamming within x secs... you lose
  (`KismetSystemLibrary.Delay` 6.0)
  (if (<= (`self.AmountPressed`) 0.0)
    (`self.OnFailed`)))

(event `PressKey`
  (set `self.AmountPressed` (`KismetMathLibrary.FClamp` (+ (`self.AmountPressed`) 1.0) 0.0 (`self.NeededAmount`)))
  (`self.UpdateProgressBar`)
  (if (== (`self.AmountPressed`) (`self.NeededAmount`))
    (`self.Completed` true)
    (`self.Destroy`)))

(event `ReleaseKey`
  (`KismetSystemLibrary.RetriggerableDelay` 0.8) ; How many seconds can the player not spam before they fail
  (`self.OnFailed`))

(event `OnFailed`
  (set `self.AmountPressed` 0.0)
  (`self.UpdateProgressBar`)
  (`self.Completed` false)
  (`self.Destroy`))

(event `Destroy`
  (bind _widgetreference (`self.WidgetReference`)
    (:`then`
      (`Widget.RemoveFromParent` _widgetreference))
    (:`else`
      _))
  (`self.K2_DestroyComponent`))

(event `Key|AnyKey`
  (params (Key :type "Key Structure"))
  (bind _returnvalue (== Key (`self.KeyPressed`)))
  (:`Pressed`
    (if _returnvalue
      (`self.PressKey`)))
  (:`Released`
    (if _returnvalue
      (`self.ReleaseKey`))))

(fn `UpdateProgressBar`
  (`ProgressBar.SetPercent` (`/Game/UI/WBP_SpamBar.SpamBar` (`self.WidgetReference`)) (/ (`self.AmountPressed`) (`self.NeededAmount`))))