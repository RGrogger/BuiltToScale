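; BP_Final_Crane is the end-of-game crane trigger that closes out play when the construction player character enters its sphere.
; The overlap teleports the character to the sphere, disables its movement and plays the PortDoor timeline, intended to swing the door mesh's yaw.
; It then shows the WBP_EndTitle widget with a fade to black and switches to UI-only input with a visible, locked cursor.
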(event `self.Sphere.OnComponentBeginOverlap`
  (params (OverlappedComponent :type "PrimitiveComponent Object Reference") (OtherActor :type "Actor Object Reference") (OtherComp :type "PrimitiveComponent Object Reference") (OtherBodyIndex :type Integer) (bFromSweep :type Boolean) (SweepResult :type "HitResult Structure (by ref)"))
  (bind _returnvalue (`GameplayStatics.GetPlayerController` 0))
  (bind _asbp_player_character_construction (cast `/Game/Core/BP_PlayerCharacter_Construction` OtherActor))
  (`self.K2_SetActorLocation` _asbp_player_character_construction (`SceneComponent.K2_GetComponentLocation` (`self.Sphere`)) false true)
  (`CharacterMovementComponent.DisableMovement` (`Character.CharacterMovement` _asbp_player_character_construction))
  (`TimelineComponent.Play` (`self.PortDoor`))
  (bind _returnvalue_2 (`|CreateWidget` "/Game/UI/WBP_EndTitle.WBP_EndTitle_C"))
  (`UserWidget.AddToViewport` _returnvalue_2 0)
  (`UserWidget.PlayAnimation` _returnvalue_2 (`/Game/UI/WBP_EndTitle.FadeToBlack` _returnvalue_2) 0.0 1 "Forward" 1.0 false)
  (`WidgetBlueprintLibrary.SetInputMode_UIOnlyEx` _returnvalue _returnvalue_2 "LockAlways")
  (set `PlayerController.bShowMouseCursor` true _returnvalue))

(fn `UserConstructionScript`)