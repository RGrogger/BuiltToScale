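; BP_Portapotty is a level checkpoint that triggers once, when a Character first overlaps its sphere.
; It plays a sound, shows the checkpoint HUD message, registers itself as the game mode's current checkpoint and enlarges the player's capsule half-height.
; A delayed timer then calls UpdateLevel, which moves the player to the tarp, increments the current level and has the player controller swap characters.
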(fn `ReceiveBeginPlay`
  (add `PrimitiveComponent.OnComponentBeginOverlap` (`self.SphereCollision`) (`|CreateDelegate` :!event `SphereBeginOverlap`)))

(fn `SphereBeginOverlap`
  (params (OverlappedComponent :type "PrimitiveComponent Object Reference") (OtherActor :type "Actor Object Reference") (OtherComp :type "PrimitiveComponent Object Reference") (OtherBodyIndex :type Integer) (bFromSweep :type Boolean) (SweepResult :type "HitResult Structure (by ref)"))
  (if (`GameplayStatics.ObjectIsA` OtherActor "/Script/Engine.Character")
    (`/Engine/EditorBlueprintResources/StandardMacros.DoOnce` false
      (:`Completed`
        ;[0 0 0] Play knocking sound + response
        (`GameplayStatics.PlaySoundAtLocation` "/Game/AnonsUsableSystem/Demo/Audio/invalid.Invalid" (+ (`self.K2_GetActorLocation`) (0.0 0.0 100.0)) (struct) 1.0 1.0 0.0 null null null null)
        ;[0 0 0] Create Message "Checkpoint Reached"
        (bind _ashud_custom (cast `/Game/UI/HUD_Custom` (`PlayerController.GetHUD` (`GameplayStatics.GetPlayerController` 0))))
        (`/Game/UI/HUD_Custom.CheckpointReached` _ashud_custom)
        ;[0 0 0] Set Player start to outside portapotty
        (bind _asgame_mode_custom (cast `/Game/Core/GameMode_Custom` (`GameplayStatics.GetGameMode`)))
        (set `/Game/Core/GameMode_Custom.CurrentCheckpoint` self _asgame_mode_custom)
        (bind _returnvalue (`GameplayStatics.GetActorOfClass` "/Game/Core/PlayerCharacter_Custom.PlayerCharacter_Custom_C"))
        (bind _capsulecomponent (`Character.CapsuleComponent` _returnvalue))
        (`CapsuleComponent.SetCapsuleHalfHeight` _capsulecomponent (+ (`CapsuleComponent.CapsuleHalfHeight` _capsulecomponent) 200.0) true)
        (`KismetSystemLibrary.K2_SetTimer` null "UpdateLevel" 5.0)))))

(fn `UpdateLevel`
  ;[0 0 0] Set Current Level
  (bind _asgame_mode_custom (cast `/Game/Core/GameMode_Custom` (`GameplayStatics.GetGameMode`)))
  (`/Game/Core/GameMode_Custom.MovePlayerToTarp` _asgame_mode_custom)
  (set `/Game/Core/GameMode_Custom.CurrentLevel` (+ (`/Game/Core/GameMode_Custom.CurrentLevel` _asgame_mode_custom) 1) _asgame_mode_custom)
  (`/Game/Core/PlayerController_Custom.SwapCharacter` (cast `/Game/Core/PlayerController_Custom` (`GameplayStatics.GetPlayerController` 0) :!pure true)))

(fn `UserConstructionScript`)