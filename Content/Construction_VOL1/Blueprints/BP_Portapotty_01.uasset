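; BP_Portapotty_01 is a portable toilet actor that acts as a level exit trigger.
; On BeginPlay it binds a handler to its sphere collision's begin overlap event.
; When a Character enters the sphere, it increments CurrentLevel on GameMode_Custom and calls InitializeLevel to set up the next level.
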(fn `ReceiveBeginPlay`
  (add `PrimitiveComponent.OnComponentBeginOverlap` (`self.SphereCollision`) (`|CreateDelegate` :!event `SphereBeginOverlap`)))

(fn `SphereBeginOverlap`
  (params (OverlappedComponent :type "PrimitiveComponent Object Reference") (OtherActor :type "Actor Object Reference") (OtherComp :type "PrimitiveComponent Object Reference") (OtherBodyIndex :type Integer) (bFromSweep :type Boolean) (SweepResult :type "HitResult Structure (by ref)"))
  (if (`GameplayStatics.ObjectIsA` OtherActor "/Script/Engine.Character")
    (bind _asgame_mode_custom (cast `/Game/Core/GameMode_Custom` (`GameplayStatics.GetGameMode`)))
    (set `/Game/Core/GameMode_Custom.CurrentLevel` (+ (`/Game/Core/GameMode_Custom.CurrentLevel` _asgame_mode_custom) 1) _asgame_mode_custom)
    (`/Game/Core/GameMode_Custom.InitializeLevel` _asgame_mode_custom)))

(fn `UserConstructionScript`)